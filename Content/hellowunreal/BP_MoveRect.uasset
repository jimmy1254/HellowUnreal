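; Actor Blueprint that moves its Cube component around a rectangular path in the relative X-Z plane.
; Tick switches on the MoveType state to step the cube right, up, left or down.
; Each side hands over to the next when the cube's relative position reaches EndPoint or drops below zero, repeating the loop.
; Steps are fixed per frame without delta-time scaling or sweep, so speed depends on frame rate.
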(event EventTick
  (params (DeltaSeconds :type Float%20%28single-precision%29))
  (bind _cube (Variables|Default|GetCube))
  (bind _cube_2 (Variables|Default|GetCube))
  (bind _cube_3 (Variables|Default|GetCube))
  (bind _cube_4 (Variables|Default|GetCube))
  (switch Utilities|FlowControl|Switch|SwitchonEN_MoveType (Variables|Default|GetMoveType)
    (:NewEnumerator0
      ;[1 1 1] 오른쪽으로 이동
      (Transformation|AddRelativeLocation _cube_4 "5.000000,0.000000,0.000000" false false)
      (if (>= (.x (Variables|/Script/Engine.SceneComponent|GetRelativeLocation _cube_4)) (Variables|Default|GetEndPoint))
        (Variables|Default|SetMoveType "NewEnumerator1")))
    (:NewEnumerator1
      ;[1 1 1] 위로 이동
      (Transformation|AddRelativeLocation _cube "0.000000,0.000000,5.000000" false false)
      (if (>= (.z (Variables|/Script/Engine.SceneComponent|GetRelativeLocation _cube)) (Variables|Default|GetEndPoint))
        (Variables|Default|SetMoveType "NewEnumerator2")))
    (:NewEnumerator2
      ;[1 1 1] 왼쪽으로 이동
      (Transformation|AddRelativeLocation _cube_2 "-5.000000,0.000000,0.000000" false false)
      (if (< (.x (Variables|/Script/Engine.SceneComponent|GetRelativeLocation _cube_2)) 0.0)
        (Variables|Default|SetMoveType "NewEnumerator3")))
    (:NewEnumerator3
      ;[1 1 1] 아래로 이동
      (Transformation|AddRelativeLocation _cube_3 "0.000000,0.000000,-5.000000" false false)
      (if (< (.z (Variables|/Script/Engine.SceneComponent|GetRelativeLocation _cube_3)) 0.0)
        (Variables|Default|SetMoveType "NewEnumerator0")))))

(fn ConstructionScript)